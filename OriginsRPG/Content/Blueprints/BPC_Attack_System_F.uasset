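; Attack component for BP_ThirdPersonCharacter that plays a four-hit melee combo, including a kick, on the character mesh from the IA_Attack input.
; When allowed, input starts the montage for the current combo index or, mid-attack, buffers the next hit.
; Each attack is DoOnce-guarded, plays after a short delay and advances the index.
; A combo-continue event, not called within this graph, consumes the buffered hit or stops and resets the combo.
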(event `self.ReceiveBeginPlay`
  (bind _asbp_third_person_character (cast `/Game/ThirdPerson/Blueprints/BP_ThirdPersonCharacter` (`self.GetOwner`)))
  (set `self.Character Mesh` (`Character.Mesh` _asbp_third_person_character)))

(event `Attack 1_F`
  ;[0.05127 0.05127 0.05127] Attack 1_F
  (`/Engine/EditorBlueprintResources/StandardMacros.DoOnce` false :!label _label
    (:`Completed`
      (`KismetSystemLibrary.Delay` 0.1)
      (`|PlayMontage` (`self.Character Mesh`) "/Game/Characters/RPG_Character/Animations/Sword_Attacks/Attack1_Montage.Attack1_Montage"
        (:`then`
          (set `self.Attack Index_F` 1)
          (goto _label :!via `Reset`))))))

(event `EnhancedInput|/Game/ThirdPerson/Input/Actions/IA_Attack`
  (params (ActionValue :type Boolean) (ElapsedSeconds :type "Float (double-precision)") (TriggeredSeconds :type "Float (double-precision)") (InputAction :type "InputAction Object Reference" :default "/Game/ThirdPerson/Input/Actions/IA_Attack.IA_Attack"))
  ;[0.05127 0.05127 0.05127] Attack Input
  (:`Started`
    (if (`self.can Attack?_F`)
      (`self.Sword Attack_F`))))

(event `Sword Attack_F`
  ;[0.05127 0.05127 0.05127] Sword Attack
  (if (`self.is Attacking?_F`)
    (set `self.save Attack_F?` true)
    (else
      (set `self.is Attacking?_F` true)
      (switch `int` (`self.Attack Index_F`) :!label _label_2
        (:`0`
          (`self.Attack 1_F`))
        (:`1`
          (`self.Attack 2_F`))
        (:`2`
          (`self.Attack 3_F`))
        (:`3`
          (`self.Attack 4_F`))))))

(event `Attack 2_F`
  ;[0.05127 0.05127 0.05127] Attack 2_F
  (`/Engine/EditorBlueprintResources/StandardMacros.DoOnce` false :!label _label_3
    (:`Completed`
      (`KismetSystemLibrary.Delay` 0.1)
      (`|PlayMontage` (`self.Character Mesh`) "/Game/Characters/RPG_Character/Animations/Sword_Attacks/Attack2_Montage.Attack2_Montage"
        (:`then`
          (set `self.Attack Index_F` 2)
          (goto _label_3 :!via `Reset`))))))

(event `Sword Attack Combo_F`
  ;[0.05127 0.05127 0.05127] Combo Continue
  (if (`self.save Attack_F?`)
    (set `self.save Attack_F?` false)
    (goto _label_2)
    (else
      (`self.Stop Combo_F`))))

(event `Attack 3_F`
  ;[0.05127 0.05127 0.05127] Attack 3_F
  (`/Engine/EditorBlueprintResources/StandardMacros.DoOnce` false :!label _label_4
    (:`Completed`
      (`KismetSystemLibrary.Delay` 0.1)
      (`|PlayMontage` (`self.Character Mesh`) "/Game/Characters/RPG_Character/Animations/Sword_Attacks/Kick_Montage.Kick_Montage"
        (:`then`
          (set `self.Attack Index_F` 3)
          (goto _label_4 :!via `Reset`))))))

(event `Stop Combo_F`
  ;[0.05127 0.05127 0.05127] Stop Combo/Attack
  (set `self.is Attacking?_F` false)
  (set `self.Attack Index_F` 0))

(event `Attack 4_F`
  ;[0.05127 0.05127 0.05127] Attack 4_F
  (`/Engine/EditorBlueprintResources/StandardMacros.DoOnce` false :!label _label_5
    (:`Completed`
      (`KismetSystemLibrary.Delay` 0.1)
      (`|PlayMontage` (`self.Character Mesh`) "/Game/Characters/RPG_Character/Animations/Sword_Attacks/Attack3_Montage.Attack3_Montage"
        (:`then`
          (set `self.Attack Index_F` 4)
          (goto _label_5 :!via `Reset`))))))